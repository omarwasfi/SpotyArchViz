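; Component that makes its owning StaticMeshActor clickable or touchable to open a mesh and material selection HUD.
; Each press registers the owner in a shared BP_GlobleVariables actor, auto-spawned if missing, then recreates the WD_HUD_Full widget.
; The Creat3DModels macro spawns BP_MeshChange3d preview actors for mesh and material options, storing them with captured photos for the selectors.
; A shared transform climbs along Z to keep previews apart.
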(event Custom|Selected%20Static%20Mesh_OnInputTouchBegin_Event
  (params (FingerIndex :type ETouchIndex%20Enum :default "Touch1") (TouchedComponent :type Primitive%20Component%20Object%20Reference))
  (CallFunction|Init)
  (bind _foundwidgets (Widget|GetAllWidgetsOfClass "/Game/MaterialChangerME/WD_HUD_Full.WD_HUD_Full_C" false))
  (for _array_element _foundwidgets
    (Widget|RemovefromParent _array_element))
  (bind _returnvalue (UserInterface|CreateWidget "/Game/MaterialChangerME/WD_HUD_Full.WD_HUD_Full_C"))
  (UserInterface|Viewport|AddtoViewport _returnvalue 0)
  (Default|SettingMaterialChangerVar _returnvalue (Utilities|Array|Get(acopy) (Variables|/Game/MaterialChangerME/BP_GlobleVariables.BP_GlobleVariables_C|GetAllParents (Variables|Default|GetGlobleVariable)) (Variables|Default|GetIndex)))
  (Default|InitMaterialSelector _returnvalue)
  (Default|InitStaticMeshSelector _returnvalue))

(event Custom|Selected%20Static%20Mesh_OnClicked_Event
  (params (TouchedComponent :type Primitive%20Component%20Object%20Reference) (ButtonPressed :type Key%20Structure))
  (CallFunction|Init)
  (bind _foundwidgets (Widget|GetAllWidgetsOfClass "/Game/MaterialChangerME/WD_HUD_Full.WD_HUD_Full_C" false))
  (for _array_element _foundwidgets
    (Widget|RemovefromParent _array_element))
  (bind _returnvalue (UserInterface|CreateWidget "/Game/MaterialChangerME/WD_HUD_Full.WD_HUD_Full_C"))
  (UserInterface|Viewport|AddtoViewport _returnvalue 0)
  (Default|SettingMaterialChangerVar _returnvalue (Utilities|Array|Get(acopy) (Variables|/Game/MaterialChangerME/BP_GlobleVariables.BP_GlobleVariables_C|GetAllParents (Variables|Default|GetGlobleVariable)) (Variables|Default|GetIndex)))
  (Default|InitMaterialSelector _returnvalue)
  (Default|InitStaticMeshSelector _returnvalue))

(event Custom|CalculateTransform
  (bind _globlevariable (Variables|Default|GetGlobleVariable))
  (Variables|Default|SetMeshTransform (Variables|/Game/MaterialChangerME/BP_GlobleVariables.BP_GlobleVariables_C|GetTransforms _globlevariable))
  (Variables|/Game/MaterialChangerME/BP_GlobleVariables.BP_GlobleVariables_C|SetTransforms _globlevariable (Math|Transform|MakeTransform (+ (.Location (Math|Transform|BreakTransform (Variables|/Game/MaterialChangerME/BP_GlobleVariables.BP_GlobleVariables_C|GetTransforms _globlevariable))) "0, 0,2000.000000") (.Rotation (Math|Transform|BreakTransform (Variables|/Game/MaterialChangerME/BP_GlobleVariables.BP_GlobleVariables_C|GetTransforms _globlevariable))) (.Scale (Math|Transform|BreakTransform (Variables|/Game/MaterialChangerME/BP_GlobleVariables.BP_GlobleVariables_C|GetTransforms _globlevariable))))))

(event Custom|GetGlobleVariable
  (bind _outactors (Actor|GetAllActorsOfClass "/Game/MaterialChangerME/BP_GlobleVariables.BP_GlobleVariables_C" :!label _label))
  (if (== (Utilities|Array|Length _outactors) 0)
    (Game|SpawnActorfromClass "/Game/MaterialChangerME/BP_GlobleVariables.BP_GlobleVariables_C" (Math|Transform|MakeTransform "0, 0, 0") "Undefined" 0 0)
    (Development|PrintString "No globle variable actor on levelplease add one")
    (goto _label)
    (else
      (Variables|Default|SetGlobleVariable (Utilities|Array|Get(acopy) _outactors)))))

(event Custom|CreatMesh
  (params (NewParam :type Static%20Mesh%20Object%20Reference))
  (bind _returnvalue (Game|SpawnActorfromClass "/Game/MaterialChangerME/BP_MeshChange3d.BP_MeshChange3d_C" (Variables|Default|GetMeshTransform) "Undefined" 0 0))
  (CallFunction|CalculateTransform)
  (Components|StaticMesh|SetStaticMesh (Variables|/Game/MaterialChangerME/BP_MeshChange3d.BP_MeshChange3d_C|GetStaticMesh _returnvalue) NewParam)
  (Default|SetTexture _returnvalue))

(event Custom|bind%20events
  (bind _asstatic_mesh_actor (Utilities|Casting|CastToStaticMeshActor (Components|GetOwner))
    (:then
      (EventDispatchers|AssignOnClicked (Variables|/Script/Engine.StaticMeshActor|GetStaticMeshComponent _asstatic_mesh_actor) (delegate Custom|Selected%20Static%20Mesh_OnClicked_Event))
      (EventDispatchers|BindEventtoOnInputTouchBegin (Variables|/Script/Engine.StaticMeshActor|GetStaticMeshComponent _asstatic_mesh_actor) (delegate Custom|Selected%20Static%20Mesh_OnInputTouchBegin_Event)))
    (:CastFailed
      (Development|PrintString "cast faild  __BP_MaterialChangerComp__ "))))

(event Custom|CreatParentActor
  (bind _returnvalue (Utilities|Array|Add (Variables|/Game/MaterialChangerME/BP_GlobleVariables.BP_GlobleVariables_C|GetAllParents (Variables|Default|GetGlobleVariable)) (Utilities|Struct|MakeST_MaterialChanger (Components|GetOwner) (Variables|Default|GetMeshes&Materials) 0 0 0 0)))
  (Variables|Default|SetIndex _returnvalue)
  (bind _asstatic_mesh_actor (Utilities|Casting|CastToStaticMeshActor (.parent (Utilities|Array|Get(acopy) (Variables|/Game/MaterialChangerME/BP_GlobleVariables.BP_GlobleVariables_C|GetAllParents (Variables|Default|GetGlobleVariable)) (Variables|Default|GetIndex))))
    (:then
      (Utilities|Creat3DModels (Variables|/Script/Engine.StaticMeshComponent|GetStaticMesh (Variables|/Script/Engine.StaticMeshActor|GetStaticMeshComponent _asstatic_mesh_actor))
        (:Done
          (bind _asmaterial (Utilities|Casting|CastToMaterial (Rendering|Material|GetMaterial (Variables|/Script/Engine.StaticMeshActor|GetStaticMeshComponent _asstatic_mesh_actor) 0)))
          (Utilities|Creat3DModels 0 _asmaterial) ; enters at MaterialsEx
        )))
    (:CastFailed
      (Development|PrintString "cast faild  __BP_MaterialChangerComp__ get globle var"))))

(event Custom|Init
  (bind _meshes_materials (Variables|Default|GetMeshes&Materials))
  (CallFunction|GetGlobleVariable)
  (CallFunction|CalculateTransform)
  (CallFunction|CreatParentActor)
  (for _array_element (.meshes _meshes_materials)
    (Utilities|Creat3DModels _array_element (stale _array_element_2)))
  (for _array_element_2 (.materials _meshes_materials)
    (Utilities|Creat3DModels _array_element _array_element_2) ; enters at MaterialsEx
  ))

(event EventBeginPlay
  (bind _asstatic_mesh_actor (Utilities|Casting|CastToStaticMeshActor (Components|GetOwner))
    (:then
      (EventDispatchers|AssignOnClicked (Variables|/Script/Engine.StaticMeshActor|GetStaticMeshComponent _asstatic_mesh_actor) (delegate Custom|Selected%20Static%20Mesh_OnClicked_Event))
      (EventDispatchers|BindEventtoOnInputTouchBegin (Variables|/Script/Engine.StaticMeshActor|GetStaticMeshComponent _asstatic_mesh_actor) (delegate Custom|Selected%20Static%20Mesh_OnInputTouchBegin_Event)))
    (:CastFailed
      (Development|PrintString "cast faild  __BP_MaterialChangerComp__ "))))