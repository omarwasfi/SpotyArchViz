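; BP_MeshChange3d is a 3D mesh preview actor that renders to a texture through a scene capture component.
; Construction creates the render target, which SetTexture and CreatPhoto bind to dynamic instances of Tex01_Mat.
; ResizeMesh recenters and uniformly scales the static mesh to a fixed bounding-sphere radius.
; From BeginPlay, a timeline repeatedly drives the Scene component's yaw, restarting whenever it finishes.
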(event Custom|SetTexture
  (bind _returnvalue (Rendering|Material|CreateDynamicMaterialInstance "/Game/MaterialChangerME/Textures/Tex-01_Mat.Tex-01_Mat" "None" :!class /Script/Engine.KismetMaterialLibrary))
  (Rendering|Material|SetTextureParameterValue _returnvalue "Texture" (Variables|Default|GetTexture))
  (Variables|Default|SetNewVar_1 _returnvalue))

(event Custom|ResizeMesh
  (bind _staticmesh (Variables|Components|GetStaticMesh))
  (bind _staticmesh_2 (Variables|/Script/Engine.StaticMeshComponent|GetStaticMesh _staticmesh))
  (bind _returnvalue (StaticMesh|GetBounds _staticmesh_2))
  (bind _returnvalue_2 (/ 2.5e+02 (.sphereradius _returnvalue)))
  (bind _returnvalue_3 (Math|Conversions|ToVector(Float) _returnvalue_2))
  ;[1 1 1] resize static mesh
  (Transformation|ResetRelativeTransform _staticmesh)
  (Class|SceneComponent|AddLocalTransform _staticmesh (Math|Transform|MakeTransform (* (* (.origin _returnvalue) -1) _returnvalue_3) "0, 0, 0" _returnvalue_3) false false))

(event EventBeginPlay
  (bind _newtrack_1 (Timeline|Timeline_0 Play)
    (:Update
      (Transformation|SetWorldRotation (Variables|Default|GetScene) (Math|Rotator|MakeRotator 0.0 0.0 _newtrack_1) false false))
    (:Finished
      (Utilities|FlowControl|Sequence
        (:then_0
          (Timeline|Timeline_0 PlayFromStart))))))

(fn ConstructionScript
  (bind _returnvalue (Rendering|CreateRenderTarget2D 1000 1000 "RTF_RGBA16f"))
  (Variables|/Script/Engine.SceneCaptureComponent2D|SetTextureTarget (Variables|Components|GetSceneCaptureComponent2D) _returnvalue)
  (Variables|Default|SetTexture _returnvalue))

(fn CreatPhoto
  (bind _returnvalue (Rendering|Material|CreateDynamicMaterialInstance "/Game/MaterialChangerME/Textures/Tex-01_Mat.Tex-01_Mat" "None" :!class /Script/Engine.KismetMaterialLibrary))
  (Rendering|Material|SetTextureParameterValue _returnvalue "Texture" (Variables|Default|GetTexture))
  (return _returnvalue))